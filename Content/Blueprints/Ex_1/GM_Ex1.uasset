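; Game mode for Exercise 1, a quiz where the player clicks which of three images matches a phrase.
; Each round shuffles Data, fills the image widget with the first three entries and shows one's text, storing its 1-based index as GoodImage.
; ClickImageEvent compares the click, shows a cached success or failure widget for two seconds, then starts another round or quits once MaxTurn is reached.
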(event Custom|ClickImageEvent
  (params (Image :type Integer))
  (if (== Image (Variables|Default|GetGoodImage))
    (|SetSuccessWidget
      (:return
        _))
    (else
      (|SetFailledWidget
        (:Return
          _))))
  (if (>= (Variables|Default|GetTurn) (Variables|Default|GetMaxTurn))
    (Game|QuitGame 0 "Quit")
    (else
      (CallFunction|SetImage)
      (CallFunction|SetText)
      (Math|Integer|IncrementInt (Variables|Default|GetTurn)))))

(event EventBeginPlay
  (Utilities|FlowControl|Sequence
    (:then_0
      (|ShowWidget))
    (:then_1
      (CallFunction|SetImage))
    (:then_2
      (CallFunction|SetText))))

(fn ConstructionScript)

(fn SetImage
  (Utilities|Array|Shuffle (Variables|Default|GetData))
  (Variables|/Game/Blueprints/Ex_1/W_Images_Ex1.W_Images_Ex1_C|SetImage1 (Variables|/Game/Blueprints/Ex_1/W_Interface_Ex1.W_Interface_Ex1_C|GetW_Images_48 (Variables|Default|GetW_Ex_1)) (.image (Utilities|Array|Get(acopy) (Variables|Default|GetData))))
  (Variables|/Game/Blueprints/Ex_1/W_Images_Ex1.W_Images_Ex1_C|SetImage2 (Variables|/Game/Blueprints/Ex_1/W_Interface_Ex1.W_Interface_Ex1_C|GetW_Images_48 (Variables|Default|GetW_Ex_1)) (.image (Utilities|Array|Get(acopy) (Variables|Default|GetData) 1)))
  (Variables|/Game/Blueprints/Ex_1/W_Images_Ex1.W_Images_Ex1_C|SetImage3 (Variables|/Game/Blueprints/Ex_1/W_Interface_Ex1.W_Interface_Ex1_C|GetW_Images_48 (Variables|Default|GetW_Ex_1)) (.image (Utilities|Array|Get(acopy) (Variables|Default|GetData) 2))))

(fn SetText
  (bind _output_get (Variables|Default|SetGoodImage (Math|Random|RandomIntegerinRange 0 2)))
  (Variables|/Game/Blueprints/Ex_1/W_Phrase_Ex1.W_Phrase_Ex1_C|SetPhrase (Variables|/Game/Blueprints/Ex_1/W_Interface_Ex1.W_Interface_Ex1_C|GetW_Phrase_65 (Variables|Default|GetW_Ex_1)) (.text (Utilities|Array|Get(acopy) (Variables|Default|GetData) _output_get)))
  (Math|Integer|IncrementInt (Variables|Default|GetGoodImage)))